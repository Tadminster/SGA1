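; Player-controlled plane pawn that constantly flies along its forward vector and banks on turn input.
; BeginPlay registers the IMC_Plane Enhanced Input mapping context, and Tick moves the actor by MoveSpeed scaled by delta time, without sweep.
; IA_Turn adds RotateSpeed-scaled input to the Body's world roll, clamped to a symmetric limit, while forcing pitch and yaw to zero.
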(event `self.ReceiveBeginPlay`
  ;[0.4375 0.4375 0.4375] Add Enhanced Input
  (bind `_as플레이어_컨트롤러` (cast `PlayerController` (`self.GetController`)))
  (bind _returnvalue (pcsubsystem `EnhancedInputLocalPlayerSubsystem` `_as플레이어_컨트롤러`))
  (`/Engine/EditorBlueprintResources/StandardMacros.IsValid` _returnvalue
    (:`Is Valid`
      (message `EnhancedInputSubsystemInterface.AddMappingContext` _returnvalue "/Game/Scene3_inflearn/Input/IMC_Plane.IMC_Plane" 0 (struct)))))

(event `self.ReceiveTick`
  (params (DeltaSeconds :type "Float (single-precision)"))
  (`self.K2_SetActorLocation` (+ (`self.K2_GetActorLocation`) (* (`self.GetActorForwardVector`) (* (`self.MoveSpeed`) DeltaSeconds)))))

(event `EnhancedInput|/Game/Scene3_inflearn/Input/IA_Turn`
  (params (ActionValue :type "Float (double-precision)") (ElapsedSeconds :type "Float (double-precision)") (TriggeredSeconds :type "Float (double-precision)") (InputAction :type "InputAction Object Reference" :default "/Game/Scene3_inflearn/Input/IA_Turn.IA_Turn"))
  (bind _returnvalue_roll (`KismetMathLibrary.BreakRotator` (`SceneComponent.K2_GetComponentRotation` (`self.Body`))))
  (:`Triggered`
    (`SceneComponent.K2_SetWorldRotation` (`self.Body`) (`KismetMathLibrary.MakeRotator` (`KismetMathLibrary.FClamp` (+ (* ActionValue (* (`self.RotateSpeed`) (`GameplayStatics.GetWorldDeltaSeconds`))) _returnvalue_roll) -45.0 45.0)) false false)))

(fn `UserConstructionScript`)