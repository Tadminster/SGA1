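; Game mode that runs the score, lives and game-over display.
; On BeginPlay it creates the BP_UI widget, adds it to the viewport and spawns an ActorSpawnManager at the world origin.
; Tick polls Score and Life, rewriting the score text and hiding life icons as lives drop.
; At zero lives it also reveals the game-over text and sets the Gameover flag.
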(event `self.ReceiveBeginPlay`
  (bind _returnvalue (`|CreateWidget` "/Game/Blueprints/BP_UI.BP_UI_C"))
  (bind _output_get (set `self.UI` _returnvalue))
  (`UserWidget.AddToViewport` _output_get 0)
  (set `self.Text Score` (`/Game/Blueprints/BP_UI.text_Score` _output_get))
  (`|SpawnActorFromClass` "/Game/Blueprints/ActorSpawnManager.ActorSpawnManager_C" (`KismetMathLibrary.MakeTransform` (0.0 0.0 0.0)) "Undefined" "MultiplyWithRoot" null null))

(event `self.ReceiveTick`
  (params (DeltaSeconds :type "Float (single-precision)"))
  (bind _ui (`self.UI`))
  (bind _life2 (`/Game/Blueprints/BP_UI.Life2` (`self.UI`)))
  (bind _life1 (`/Game/Blueprints/BP_UI.Life1` _ui))
  (bind _life3 (`/Game/Blueprints/BP_UI.Life3` (`self.UI`)))
  (`TextBlock.SetText` (`self.Text Score`) (`KismetTextLibrary.Conv_StringToText` (`KismetStringLibrary.Concat_StrStr` "Score: " (`KismetStringLibrary.Conv_IntToString` (`self.score`)))))
  (switch `int` (`self.life`)
    (:`0`
      (if (`Widget.IsVisible` _life1)
        (set `Widget.Visibility` "Hidden" _life1)
        (set `Widget.Visibility` "Visible" (`/Game/Blueprints/BP_UI.text_gameover` _ui))
        (set `self.bGameover` true)))
    (:`1`
      (if (`Widget.IsVisible` _life2)
        (set `Widget.Visibility` "Hidden" _life2)))
    (:`2`
      (if (`Widget.IsVisible` _life3)
        (set `Widget.Visibility` "Hidden" _life3)))))

(fn `UserConstructionScript`)