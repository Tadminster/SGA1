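; Red cube obstacle that moves along world X and damages the player on contact.
; BeginPlay caches NewGameMode and BP_Player via GetActorOfClass.
; While the game is not over, Tick lowers Speed by DeltaSeconds and applies it as a per-frame X offset, so velocity steadily shifts toward negative X.
; Any mesh overlap, unfiltered by actor, decrements GameMode Life, sets the player's TakeDamage flag and destroys the cube.
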(event `self.ReceiveBeginPlay`
  (`|ExecutionSequence`
    (:`then_0`
      (bind _returnvalue (`GameplayStatics.GetActorOfClass` "/Game/Blueprints/NewGameMode.NewGameMode_C"))
      (set `self.gameMode` _returnvalue))
    (:`then_1`
      (bind _returnvalue_2 (`GameplayStatics.GetActorOfClass` "/Game/Blueprints/BP_Player.BP_Player_C"))
      (set `self.player` _returnvalue_2))))

(event `self.ReceiveTick`
  (params (DeltaSeconds :type "Float (single-precision)"))
  (if (not (`/Game/Blueprints/NewGameMode.bGameover` (`self.gameMode`)))
    (bind _output_get (set `self.speed` (- (`self.speed`) DeltaSeconds)))
    (`self.K2_AddActorWorldOffset` (`KismetMathLibrary.MakeVector` _output_get))))

(event `self.StaticMesh.OnComponentBeginOverlap`
  (params (OverlappedComponent :type "PrimitiveComponent Object Reference") (OtherActor :type "Actor Object Reference") (OtherComp :type "PrimitiveComponent Object Reference") (OtherBodyIndex :type Integer) (bFromSweep :type Boolean) (SweepResult :type "HitResult Structure (by ref)"))
  (bind _gamemode (`self.gameMode`))
  (set `/Game/Blueprints/NewGameMode.life` (- (`/Game/Blueprints/NewGameMode.life` _gamemode) 1) _gamemode)
  (set `/Game/Blueprints/BP_Player.bTakeDamage` true (`self.player`))
  (`self.K2_DestroyActor`))

(fn `UserConstructionScript`)