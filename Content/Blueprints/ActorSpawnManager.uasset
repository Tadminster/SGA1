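; ActorSpawnManager feeds a lane-based obstacle game by spawning random obstacles ahead on the track.
; BeginPlay caches the NewGameMode actor, and Tick checks its Gameover flag to stop spawning.
; A Delay on Tick throttles spawning to a steady interval, since repeated calls are ignored while it runs.
; Each spawn randomly picks a green cube, red cube or BP_Line and one of three lanes at a fixed forward position.
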(event `self.ReceiveBeginPlay`
  (bind _returnvalue (`GameplayStatics.GetActorOfClass` "/Game/Blueprints/NewGameMode.NewGameMode_C"))
  (set `self.gameMode` _returnvalue))

(event `self.ReceiveTick`
  (params (DeltaSeconds :type "Float (single-precision)"))
  (bind _returnvalue (`KismetMathLibrary.MakeTransform` (`KismetMathLibrary.MakeVector` 2000.0 (`KismetMathLibrary.Conv_IntToDouble` (* (`KismetMathLibrary.RandomIntegerInRange` -1 1) 200)) 100.0) (struct) (0.4 0.4 0.4)))
  (if (not (`/Game/Blueprints/NewGameMode.bGameover` (`self.gameMode`)))
    (`KismetSystemLibrary.Delay` 2.0)
    (switch `int` (`KismetMathLibrary.RandomIntegerInRange` 0 2)
      (:`0`
        (`|SpawnActorFromClass` "/Game/Blueprints/BP_Obstacle_GreenCube.BP_Obstacle_GreenCube_C" _returnvalue "Undefined" "MultiplyWithRoot" null null))
      (:`1`
        (`|SpawnActorFromClass` "/Game/Blueprints/BP_Obstacle_RedCube.BP_Obstacle_RedCube_C" _returnvalue "Undefined" "MultiplyWithRoot" null null))
      (:`2`
        (`|SpawnActorFromClass` "/Game/Blueprints/BP_Line.BP_Line_C" _returnvalue "Undefined" "MultiplyWithRoot" null null)))))

(fn `UserConstructionScript`)