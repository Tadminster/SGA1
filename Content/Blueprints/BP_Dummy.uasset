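; BP_Dummy is a damageable dummy character that reacts to overlaps on its capsule component.
; When TakeDamage is false, an overlap plays a hit montage, subtracts random damage from HitPoint clamped at zero, and prints the result.
; It also spawns a DamageDisplay actor at a slightly jittered position, whose number is rolled separately and can differ from the damage applied.
; TakeDamage is never set in this graph.
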(event `self.CapsuleComponent.OnComponentBeginOverlap`
  (params (OverlappedComponent :type "PrimitiveComponent Object Reference") (OtherActor :type "Actor Object Reference") (OtherComp :type "PrimitiveComponent Object Reference") (OtherBodyIndex :type Integer) (bFromSweep :type Boolean) (SweepResult :type "HitResult Structure (by ref)"))
  (bind _returnvalue (`KismetMathLibrary.RandomIntegerInRange` 8 12))
  (if (not (`self.bTakeDamage`))
    (`self.PlayAnimMontage` "/Game/Characters/Mannequins/Animations/Manny/AM_TakeDamage.AM_TakeDamage")
    (set `self.hitPoint` (`KismetMathLibrary.Max` (- (`self.hitPoint`) _returnvalue)))
    (bind _returnvalue_2 (`|SpawnActorFromClass` "/Game/Blueprints/DamageDisplay.DamageDisplay_C" (`KismetMathLibrary.MakeTransform` (+ (`self.K2_GetActorLocation`) (`KismetMathLibrary.MakeVector` (`KismetMathLibrary.RandomFloatInRange` -2.0 2.0) (`KismetMathLibrary.RandomFloatInRange` -2.0 2.0) (`KismetMathLibrary.RandomFloatInRange` 2.0 4.0)))) "Undefined" "MultiplyWithRoot" null null))
    (`TextRenderComponent.K2_SetText` (`/Game/Blueprints/DamageDisplay.TextRender` _returnvalue_2) (`KismetTextLibrary.Conv_IntToText` _returnvalue))
    (`KismetSystemLibrary.PrintString` (`KismetStringLibrary.Conv_IntToString` (`self.hitPoint`)))))

(fn `UserConstructionScript`)