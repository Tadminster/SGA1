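; Green cube obstacle actor that moves along world X and awards a point when its mesh is overlapped.
; BeginPlay caches NewGameMode via GetActorOfClass for the shared Gameover flag and Score.
; Until game over, Tick lowers Speed by delta time and applies it as a per-frame X offset, unscaled by delta time.
; Any mesh overlap increments and prints Score, then destroys the cube, without checking the other actor.
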(event `self.ReceiveBeginPlay`
  (bind _returnvalue (`GameplayStatics.GetActorOfClass` "/Game/Blueprints/NewGameMode.NewGameMode_C"))
  (set `self.gameMode` _returnvalue))

(event `self.ReceiveTick`
  (params (DeltaSeconds :type "Float (single-precision)"))
  (if (not (`/Game/Blueprints/NewGameMode.bGameover` (`self.gameMode`)))
    (bind _output_get (set `self.speed` (- (`self.speed`) DeltaSeconds)))
    (`self.K2_AddActorWorldOffset` (`KismetMathLibrary.MakeVector` _output_get))))

(event `self.StaticMesh.OnComponentBeginOverlap`
  (params (OverlappedComponent :type "PrimitiveComponent Object Reference") (OtherActor :type "Actor Object Reference") (OtherComp :type "PrimitiveComponent Object Reference") (OtherBodyIndex :type Integer) (bFromSweep :type Boolean) (SweepResult :type "HitResult Structure (by ref)"))
  (bind _gamemode (`self.gameMode`))
  (bind _output_get (set `/Game/Blueprints/NewGameMode.score` (+ (`/Game/Blueprints/NewGameMode.score` _gamemode) 1) _gamemode))
  (`KismetSystemLibrary.PrintText` (`KismetTextLibrary.Conv_IntToText` _output_get))
  (`self.K2_DestroyActor`))

(fn `UserConstructionScript`)